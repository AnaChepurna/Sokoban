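; Test actor that snaps itself to a 120-unit XY grid and relays overlap events to its Transfer member.
; The construction script fixes Z at 100, resets rotation and scale, and derives X and Y through RoundLocation, which keeps whole multiples of the cell size rather than rounding to nearest.
; Actor begin and end overlaps pass the other actor straight to Transfer; the Cube bounds-scale call is unconnected.
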(event Collision|EventActorBeginOverlap
  (params (OtherActor :type Actor%20Object%20Reference))
  (Class|TransferComponent|OnBeginOverlap (Variables|Default|GetTransfer) OtherActor))

(event Collision|EventActorEndOverlap
  (params (OtherActor :type Actor%20Object%20Reference))
  (Class|TransferComponent|OnEndOverlap (Variables|Default|GetTransfer) OtherActor))

(fn ConstructionScript
  (bind _returnvalue (Transformation|GetActorLocation))
  (bind (_x _y) (Math|Vector|BreakVector _returnvalue))
  (Transformation|SetActorTransform (Math|Transform|MakeTransform (Math|Vector|MakeVector (CallFunction|RoundLocation _x 1.2e+02) (CallFunction|RoundLocation _y 1.2e+02) 1e+02))))

(fn RoundLocation
  (params (Value :type Float%20%28single-precision%29) (size :type Float%20%28single-precision%29))
  (return (* (Math|Conversions|ToFloat(Integer) (.ReturnValue (Math|Float|Division(WholeandRemainder) Value size))) size)))