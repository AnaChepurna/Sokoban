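; BP_Test is a grid-snapped test actor that forwards its begin and end overlap events to a Transfer member.
; Its construction script resets rotation and scale, fixes the height, and snaps X and Y to a 120-unit grid using whole-number division.
; It then traces downward for static or dynamic world objects and destroys itself if nothing is below.
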(event Collision|EventActorBeginOverlap
  (params (OtherActor :type Actor%20Object%20Reference))
  (Class|TransferComponent|OnBeginOverlap (Variables|Default|GetTransfer) OtherActor))

(event Collision|EventActorEndOverlap
  (params (OtherActor :type Actor%20Object%20Reference))
  (Class|TransferComponent|OnEndOverlap (Variables|Default|GetTransfer) OtherActor))

(fn ConstructionScript
  (bind _returnvalue (Transformation|GetActorLocation))
  (bind _returnvalue_2 (Transformation|GetActorLocation))
  (bind (_x _y) (Math|Vector|BreakVector _returnvalue))
  (Utilities|FlowControl|Sequence
    (:then_0
      (Transformation|SetActorTransform (Math|Transform|MakeTransform (Math|Vector|MakeVector (CallFunction|RoundLocation _x 1.2e+02) (CallFunction|RoundLocation _y 1.2e+02) 6e+01))))
    (:then_1
      (bind _returnvalue_3 (Collision|LineTraceForObjects _returnvalue_2 (+ _returnvalue_2 "0.000000, 0,-100.000000") (Utilities|Array|MakeArray "ObjectTypeQuery1" "ObjectTypeQuery2") false 0 "None"))
      (if (not _returnvalue_3)
        (Actor|DestroyActor)))))

(fn RoundLocation
  (params (Value :type Float%20%28single-precision%29) (size :type Float%20%28single-precision%29))
  (return (* (Math|Conversions|ToFloat(Integer) (.ReturnValue (Math|Float|Division(WholeandRemainder) Value size))) size)))